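; A placed map actor that snaps the first player controller's spectator pawn to its own location and rotation, serving as a spectator camera fix.
; On BeginPlay it polls with a short delay until that spectator pawn is valid.
; It then applies the transform, re-applies rotation, and finally teleports location and rotation, with brief delays between these repeated passes.
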(event EventBeginPlay
  (bind _returnvalue (Game|GetPlayerController 0))
  (bind _returnvalue_2 (Transformation|GetActorRotation))
  (bind _returnvalue_3 (Pawn|GetSpectatorPawn _returnvalue))
  ;[1 1 1] Get client's Spectator Camera. If it exists, move it. If not, try and find it again.
  (Utilities|IsValid _returnvalue_3 :!label _label ; Are they in control of a spectator?
    (:Is%20Valid
      (Transformation|SetActorTransform _returnvalue_3 (Transformation|GetActorTransform))
      (Utilities|FlowControl|Delay 0.2)
      (Transformation|SetActorRotation _returnvalue_3 _returnvalue_2)
      (Utilities|FlowControl|Delay 0.2)
      (Transformation|SetActorLocationAndRotation _returnvalue_3 (Transformation|GetActorLocation) _returnvalue_2 false true))
    (:Is%20Not%20Valid
      (Utilities|FlowControl|Delay 0.02)
      (goto _label))))

(fn ConstructionScript)