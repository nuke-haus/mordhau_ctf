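; Game mode for Capture the Flag that resets flag pedestals at start and handles captures, announcements and match end.
; A capture awards the player points, plays a sound, announces it on all HUDs and decrements the opposing team's score.
; When a team's score changes from zero, the authority disables scoring, ends the match and shows local players victory or defeat.
; ForceEndGame ends it directly, also allowing draws; the wait-for-both-teams start logic is disconnected.
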(event Custom|GameEndingEvent
  (params (Team :type Integer))
  (for _index (range 0 (stale _returnvalue))
    (if (and (Utilities|IsValid (Game|GetPlayerController _index)) (Pawn|IsLocalPlayerController (Game|GetPlayerController _index)))
      (bind _asbp_mordhau_hud (Utilities|Casting|CastToBP_MordhauHUD (HUD|GetHUD (Game|GetPlayerController _index))))
      (bind _asbp_mordhau_player_state (Utilities|Casting|CastToBP_MordhauPlayerState (Variables|/Script/Engine.Controller|GetPlayerState (Game|GetPlayerController _index))))
      (if (== Team 2)
        (Default|ShowMatchResult _asbp_mordhau_hud false "draw")
        (elif (== (Variables|/Script/Mordhau.MordhauPlayerState|GetTeam _asbp_mordhau_player_state) Team)
          (Default|ShowMatchResult _asbp_mordhau_hud true "victory")
          (else
            (Default|ShowMatchResult _asbp_mordhau_hud false "defeat")))))))

(event Custom|Announce
  (params (Announcement :type Text) (SubText :type Text) (Duration :type Float%20%28single-precision%29) (PlayDing :type Boolean) (PlayDong :type Boolean))
  (if PlayDong
    (Audio|Components|Audio|Play (Variables|Default|GetDong) 0.0))
  (if PlayDing
    (Audio|Components|Audio|Play (Variables|Default|GetDing) 0.0))
  (bind _outactors (Actor|GetAllActorsOfClass "/Game/Mordhau/Blueprints/BP_MordhauPlayerController.BP_MordhauPlayerController_C"))
  (for _array_element _outactors
    (bind _asbp_mordhau_hud (Utilities|Casting|CastToBP_MordhauHUD (HUD|GetHUD _array_element)))
    (Default|ShowAnnouncement _asbp_mordhau_hud Announcement SubText Duration)))

(event Custom|Capture
  (params (Team :type Byte) (Character :type Mordhau%20Character%20Object%20Reference))
  (bind _asmordhau_player_controller (Utilities|Casting|CastToMordhauPlayerController (Pawn|GetController Character)))
  (Class|MordhauPlayerController|ClientReceiveScoreBP _asmordhau_player_controller "Captured" 0 3e+02)
  (bind _asbp_mordhau_player_state (Utilities|Casting|CastToBP_MordhauPlayerState (Variables|/Script/Engine.Pawn|GetPlayerState Character)))
  (Class|MordhauPlayerState|AddScore _asbp_mordhau_player_state 300)
  (Audio|Components|Audio|Play (Variables|Default|GetCaptureSound) 0.0)
  (switch int (Math|Conversions|ToInteger(Byte) Team)
    (:Default
      (CallFunction|Announce "BLUE TEAM CAPTURED THE FLAG" "" 3.0 false false :!label _label)
      (Class|MordhauGameMode|AddTeamScore 0 -1.0))
    (:0
      (CallFunction|Announce "RED TEAM CAPTURED THE FLAG" "" 3.0 false false)
      (Class|MordhauGameMode|AddTeamScore 1 -1.0))
    (:1
      (goto _label))))

(event EventBeginPlay
  (|CallParentFunction)
  (bind _outactors (Actor|GetAllActorsOfClass "/Game/Mordhau/Maps/Sandstorm/Sandstorm_sharedassets/CTF/FlagPedestal.FlagPedestal_C"))
  (for _array_element _outactors
    (Default|Reset _array_element)))

(event EventTick
  (params (DeltaSeconds :type Float%20%28single-precision%29)))

(event EventOnTeamScoreChanged
  (params (Team :type Integer) (OldValue :type Float%20%28single-precision%29))
  (bind _self self)
  (Networking|SwitchHasAuthority
    (:Authority
      (Utilities|Casting|CastToBP_CTFGameState (Game|GetGameState))
      (switch int Team
        (:0
          (if (Math|Float|NearlyEqual(Float) OldValue 0.0 0.01)
            (Variables|Default|SetbIsScoringDisabled true)
            (Utilities|FlowControl|Delay 0.2)
            (Class|GameMode|EndMatch _self)
            (CallFunction|GameEndingEvent 1)))
        (:1
          (if (Math|Float|NearlyEqual(Float) OldValue 0.0 0.01)
            (Variables|Default|SetbIsScoringDisabled true)
            (Utilities|FlowControl|Delay 0.2)
            (Class|GameMode|EndMatch _self)
            (CallFunction|GameEndingEvent)))))))

(fn ConstructionScript
  (|CallParentFunction))

(fn ForceEndGame
  (params (WinnerTeam :type Integer))
  (Class|GameMode|EndMatch self)
  (CallFunction|GameEndingEvent WinnerTeam))