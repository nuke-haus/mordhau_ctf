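; Game mode for Mordhau capture-the-flag that handles flag captures, team scoring and the match win.
; Capture announces the scoring team and adds a point; when that team reaches ScoreToWin, the authority disables scoring and, after a delay, ends the match with the winner screen.
; It resets flag pedestals at BeginPlay, refreshes flag widgets on PostLogin and drops carried flags on death.
; The restart-once-both-teams-have-players logic is disconnected.
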(event Custom|Capture
  (params (Team :type Byte))
  (bind _returnvalue (Game|GetGameState))
  (bind _asbp_ctfgame_state (Utilities|Casting|CastToBP_CTFGameState (Game|GetGameState)))
  (switch int (Math|Conversions|ToInteger(Byte) Team)
    (:Default
      (Default|DoAnnounce _asbp_ctfgame_state "BLUE TEAM CAPTURED THE FLAG" "" 3.0 :!label _label)
      (Class|MordhauGameMode|AddTeamScore 1 1.0)
      (bind _asbp_mordhau_game_state (Utilities|Casting|CastToBP_MordhauGameState _returnvalue))
      (CallFunction|TeamScoreUpdated 1 (Utilities|Array|Get(acopy) (Variables|/Script/Mordhau.MordhauGameState|GetTeamScores _asbp_mordhau_game_state) 1)))
    (:0
      (Default|DoAnnounce _asbp_ctfgame_state "RED TEAM CAPTURED THE FLAG" "" 3.0)
      (Class|MordhauGameMode|AddTeamScore 0 1.0)
      (bind _asbp_mordhau_game_state_2 (Utilities|Casting|CastToBP_MordhauGameState _returnvalue))
      (CallFunction|TeamScoreUpdated 0 (Utilities|Array|Get(acopy) (Variables|/Script/Mordhau.MordhauGameState|GetTeamScores _asbp_mordhau_game_state_2))))
    (:1
      (goto _label))))

(event Custom|TeamScoreUpdated
  (params (Team :type Integer) (Score :type Float%20%28single-precision%29))
  (bind _scoretowin (Variables|Default|GetScoreToWin))
  (bind _returnvalue (Math|Float|NearlyEqual(Float) Score _scoretowin 0.01))
  (Networking|SwitchHasAuthority
    (:Authority
      (Utilities|Casting|CastToBP_CTFGameState (Game|GetGameState))
      (switch int Team
        (:0
          (if _returnvalue
            (Variables|Default|SetbIsScoringDisabled true)
            (Utilities|FlowControl|Delay 5.0)
            (CallFunction|ForceEndGame)))
        (:1
          (if _returnvalue
            (Variables|Default|SetbIsScoringDisabled true)
            (Utilities|FlowControl|Delay 5.0)
            (CallFunction|ForceEndGame 1)))))))

(event EventBeginPlay
  (|CallParentFunction)
  (bind _outactors (Actor|GetAllActorsOfClass "/Game/Mordhau/Maps/NukeCTF/FlagPedestal.FlagPedestal_C"))
  (for _array_element _outactors
    (Default|Reset _array_element false)))

(event EventTick
  (params (DeltaSeconds :type Float%20%28single-precision%29)))

(event EventPostLogin
  (params (NewPlayer :type Player%20Controller%20Object%20Reference))
  (bind _outactors (Actor|GetAllActorsOfClass "/Game/Mordhau/Maps/NukeCTF/FlagPedestal.FlagPedestal_C"))
  (for _array_element _outactors
    (bind _asctfflag (Utilities|Casting|CastToCTFFlag (Variables|/Game/Mordhau/Maps/NukeCTF/FlagPedestal.FlagPedestal_C|GetFlag _array_element)))
    (Utilities|IsValid _asctfflag
      (:Is%20Valid
        (Default|SetWidgetData _asctfflag (Math|Conversions|ToInteger(Byte) (Variables|/Game/Mordhau/Maps/NukeCTF/FlagPedestal.FlagPedestal_C|GetTeam _array_element)))))))

(event EventOnTeamScoreChanged
  (params (Team :type Integer) (OldValue :type Float%20%28single-precision%29)))

(event EventOnKilled
  (params (Killer :type Controller%20Object%20Reference) (KilledPlayer :type Controller%20Object%20Reference) (KilledPawn :type Pawn%20Object%20Reference) (Type :type EMordhauDamageType%20Enum :default "Generic") (SubType :type Byte :default 0) (DamageSource :type Actor%20Object%20Reference) (DamageAgent :type Actor%20Object%20Reference))
  (Utilities|FlowControl|Sequence
    (:then_0
      (bind _asmordhau_character (Utilities|Casting|CastToMordhauCharacter KilledPawn))
      (for _array_element (Variables|/Script/Mordhau.MordhauCharacter|GetEquipment _asmordhau_character)
        (if (== (Utilities|GetClass _array_element) "/Game/Mordhau/Maps/NukeCTF/CTFFlag.CTFFlag_C")
          (Class|MordhauCharacter|DropEquipment _asmordhau_character _array_element))))
    (:then_1
      (|CallParentFunction Killer KilledPlayer KilledPawn Type SubType DamageSource DamageAgent))))

(fn ConstructionScript
  (|CallParentFunction))

(fn ForceEndGame
  (params (WinnerTeam :type Integer))
  (Class|GameMode|EndMatch self)
  (bind _asbp_ctfgame_state (Utilities|Casting|CastToBP_CTFGameState (Game|GetGameState)))
  (Default|DoEndGameScreen _asbp_ctfgame_state WinnerTeam))