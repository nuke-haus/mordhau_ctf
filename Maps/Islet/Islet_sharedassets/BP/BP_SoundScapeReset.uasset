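; Map trigger actor for Islet that resets the soundscape when the locally controlled Mordhau character overlaps its Cube.
; On overlap it fades out SoundsToDisable and fades in or re-levels SoundsToEnable using per-index VolumeScales.
; Each audio component's SuppressSubtitles flag is repurposed as a playing marker to avoid restarting active sounds.
; From BeginPlay, the actor endlessly sweeps 500 units up and back down at short intervals.
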(event OnComponentBeginOverlap(Cube)
  (params (OverlappedComponent :type Primitive%20Component%20Object%20Reference) (OtherActor :type Actor%20Object%20Reference) (OtherComp :type Primitive%20Component%20Object%20Reference) (OtherBodyIndex :type Integer) (bFromSweep :type Boolean) (SweepResult :type Hit%20Result%20Structure%20%28by%20ref%29))
  (bind _asbp_mordhau_character (Utilities|Casting|CastToBP_MordhauCharacter OtherActor))
  (if (Pawn|IsLocallyControlled _asbp_mordhau_character)
    (for _array_element (Variables|Default|GetSoundsToDisable)
      (Audio|Components|Audio|FadeOut (Variables|/Script/Engine.AmbientSound|GetAudioComponent _array_element) 2.0 0.0 :!class /Script/Engine.AudioComponent)
      (Variables|/Script/Engine.AudioComponent|SetbSuppressSubtitles (Variables|/Script/Engine.AmbientSound|GetAudioComponent _array_element) false))
    (for (_array_element_2 _array_index) (Variables|Default|GetSoundsToEnable)
      (if (Variables|/Script/Engine.AudioComponent|GetbSuppressSubtitles (Variables|/Script/Engine.AmbientSound|GetAudioComponent _array_element_2))
        (Audio|Components|Audio|AdjustVolume (Variables|/Script/Engine.AmbientSound|GetAudioComponent _array_element_2) 2.0 (Utilities|Array|Get(acopy) (Variables|Default|GetVolumeScales) _array_index) :!class /Script/Engine.AudioComponent)
        (else
          (Audio|Components|Audio|FadeIn (Variables|/Script/Engine.AmbientSound|GetAudioComponent _array_element_2) 2.0 (Utilities|Array|Get(acopy) (Variables|Default|GetVolumeScales) _array_index) 0.0 :!class /Script/Engine.AudioComponent)
          (Variables|/Script/Engine.AudioComponent|SetbSuppressSubtitles (Variables|/Script/Engine.AmbientSound|GetAudioComponent _array_element_2) true))))))

(event EventBeginPlay
  (Transformation|SetActorLocation (+ (Transformation|GetActorLocation self) "0, 0,500.000000") true false :!label _label)
  (Utilities|FlowControl|Delay 0.3)
  (Transformation|SetActorLocation (+ (Transformation|GetActorLocation self) "0, 0,-500.000000") true false)
  (Utilities|FlowControl|Delay 0.3)
  (goto _label))

(event Collision|EventActorBeginOverlap
  (params (OtherActor :type Actor%20Object%20Reference)))

(event EventTick
  (params (DeltaSeconds :type Float%20%28single-precision%29)))

(fn ConstructionScript)