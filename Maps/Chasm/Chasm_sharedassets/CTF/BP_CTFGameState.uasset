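; Game state for Capture the Flag on Chasm, running a timed match decided by team score.
; BeginPlay sets the stage end time and, on authority, seeds both team scores.
; Tick handles one-time ammo box and equipment cleanup, warmup announcements, objective and post-match HUD, then has BP_CTFGameMode end the game on timeout by comparing scores.
; The scoreboard shows time remaining; Frontline/Push ticket and capture logic remains disconnected.
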(event Custom|TriggerWinDelayed)

(event EventBeginPlay
  (bind _returnvalue (Utilities|Time|GetTimeSeconds))
  (bind _initialstagetime (Variables|Default|GetInitialStageTime))
  (bind _teamscores (Variables|Default|GetTeamScores))
  (bind _returnvalue_2 (+ _returnvalue _initialstagetime))
  (Variables|Default|SetMatchDurationMax (Math|Float|Truncate _returnvalue_2))
  (Variables|Default|SetStageEndTime _returnvalue_2)
  (Variables|Default|SetAllObjectivesCompletedTime 0.0)
  (Networking|SwitchHasAuthority
    (:Authority
      (Utilities|FlowControl|DoOnce false
        (:Completed
          (Utilities|Array|SetArrayElem _teamscores 0 (Variables|Default|GetTeam1StartingTickets))
          (Utilities|Array|SetArrayElem _teamscores 1 (Variables|Default|GetTeam2StartingTickets)))))))

(event EventLocalPlayerChangedTeam
  (|CallParentFunction))

(event EventTick
  (params (DeltaSeconds :type Float%20%28single-precision%29))
  (bind _returnvalue (Game|GetPlayerController 0))
  (bind _returnvalue_2 (GameState|GetServerWorldTimeSeconds))
  (bind _teamscores (Variables|Default|GetTeamScores))
  (bind _warmupend (Variables|Default|GetWarmupEnd))
  (bind _returnvalue_3 (- _warmupend _returnvalue_2))
  (bind _returnvalue_4 (Math|Float|Max(Float) _returnvalue_3 0.0))
  (bind _returnvalue_5 (Math|Float|Ceil _returnvalue_4))
  (Utilities|FlowControl|Sequence
    (:then_0
      (Utilities|FlowControl|DoOnce false
        (:Completed
          (Utilities|FlowControl|Delay 0.05)
          (Utilities|FlowControl|Sequence
            (:then_0
              (if (Variables|Default|GetNoAmmoBoxes)
                (bind _outactors (Actor|GetAllActorsOfClass "/Game/Mordhau/Blueprints/Interactables/Environment/Specific/BP_AmmoBox.BP_AmmoBox_C"))
                (for _array_element _outactors
                  (Actor|DestroyActor _array_element))))
            (:then_1
              (Networking|SwitchHasAuthority
                (:Authority
                  (if (Variables|Default|GetNoPreplacedEquipment)
                    (bind _outactors_2 (Actor|GetAllActorsOfClass "/Script/Mordhau.MordhauEquipment"))
                    (for _array_element_2 _outactors_2
                      (Actor|DestroyActor _array_element_2))))))))))
    (:then_1
      (bind _asbp_mordhau_player_controller (Utilities|Casting|CastToBP_MordhauPlayerController _returnvalue))
      (if (Pawn|IsLocalPlayerController _returnvalue)
        (bind _asbp_mordhau_hud (Utilities|Casting|CastToBP_MordhauHUD (HUD|GetHUD _returnvalue)))
        (switch name (Variables|Default|GetMatchState)
          (:WaitingToStart
            ;[1 1 1] WaitingToStart
            (Utilities|Casting|CastToAdvancedCharacter (Pawn|GetControlledPawn _returnvalue))
            (if (!= _warmupend -1.0)
              (if (!= _returnvalue_5 0)
                (Default|ShowAnnouncement _asbp_mordhau_hud "Match starting" (Utilities|Text|FormatText "-{0}-" _returnvalue_5) 0.1))
              (else
                (Default|ShowAnnouncement _asbp_mordhau_hud "Waiting for players" "" 0.1))))
          (:WaitingPostMatch
            ;[1 1 1] WaitingPostMatch
            (Utilities|FlowControl|DoOnce (Variables|Default|GetbDoNotGoToNextMapOnMatchEnd)
              (:Completed
                (if (not (Variables|Default|GetbDoNotShowPostMatchScreen))
                  (Utilities|FlowControl|Delay (Variables|Default|GetPostMatchScreenDelay))
                  (Default|HideScoreboard _asbp_mordhau_hud)
                  (bind _asbp_mordhau_hud_2 (Utilities|Casting|CastToBP_MordhauHUD (HUD|GetHUD _asbp_mordhau_player_controller)))
                  (Default|ShowPostMatchScreen _asbp_mordhau_hud_2))))))))
    (:then_2
      (Utilities|FlowControl|Sequence
        (:then_0
          (Networking|CanExecuteCosmeticEvents
            (:True
              (if (Class|GameStateBase|HasMatchStarted)
                (Utilities|FlowControl|DoOnce false
                  (:Completed
                    (bind _asbp_frontline_player_controller (Utilities|Casting|CastToBP_FrontlinePlayerController (Game|GetPlayerController 0)))
                    (bind _asbp_frontline_hud (Utilities|Casting|CastToBP_FrontlineHUD (Class|MordhauUtilityLibrary|GetMordhauHUD)))
                    (Default|ShowObjectives _asbp_frontline_hud)
                    (bind _asbp_push_player_controller (Utilities|Casting|CastToBP_PushPlayerController _asbp_frontline_player_controller))
                    (Default|ShowCurrentObjective _asbp_push_player_controller true)))))))
        (:then_1
          (Math|Float|CompareFloat (Variables|Default|GetStageEndTime) (Utilities|Time|GetTimeSeconds)
            (:<
              (Utilities|FlowControl|DoOnce false
                (:Completed
                  (bind _asbp_ctfgame_mode (Utilities|Casting|CastToBP_CTFGameMode (Game|GetGameMode)))
                  (Math|Float|CompareFloat (Utilities|Array|Get(acopy) _teamscores) (Utilities|Array|Get(acopy) _teamscores 1)
                    (:>
                      (Default|ForceEndGame _asbp_ctfgame_mode))
                    (:==
                      (Default|ForceEndGame _asbp_ctfgame_mode 2))
                    (:<
                      (Default|ForceEndGame _asbp_ctfgame_mode 1))))))))))))

(fn ConstructionScript
  (|CallParentFunction))

(fn DrainTix
  (params (Game :type BP%20Mordhau%20Game%20Mode%20Object%20Reference))
  (bind _teamscores (Variables|Default|GetTeamScores))
  (Utilities|FlowControl|Sequence
    (:then_0
      (Variables|Default|SetTeam%200%20Score (Utilities|Array|Get(acopy) _teamscores))
      (Variables|Default|SetTeam%201%20Score (Utilities|Array|Get(acopy) _teamscores 1)))
    (:then_1
      (if (and (<= (Variables|Default|GetTeam%200%20Score) 0.0) (<= (Variables|Default|GetTeam%201%20Score) 0.0))
        ;[1 1 1] Draw
        (Class|GameMode|EndMatch Game)
        (Variables|Default|SetMatchEndInfo (Utilities|Struct|MakeSTRUCT_MatchEndInfo 0 0 0.0 0.0 true)))
      (Class|MordhauGameMode|SetTeamScore Game 0 (Math|Float|Max(Float) (Variables|Default|GetTeam%200%20Score) 0.0))
      (Class|MordhauGameMode|SetTeamScore Game 1 (Math|Float|Max(Float) (Variables|Default|GetTeam%201%20Score) 0.0)))))

(fn GetScoreboardTimeinProgress
  (return (Math|Timespan|FromSeconds (Math|Float|Max(Float) (- (Variables|Default|GetStageEndTime) (GameState|GetServerWorldTimeSeconds)) 0.0))))