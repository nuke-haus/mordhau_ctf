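; BP_CTFHUD is the HUD for Capture the Flag on the Chasm map, extending a parent HUD class.
; When the game state replicates, it removes the parent's Push and Frontline widgets and adds a CTF widget at a negative Z-order, hidden if minimal HUD is active.
; Overrides of the main menu and minimal/full HUD events run parent logic, then toggle that widget's visibility.
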(event EventBeginPlay
  (|CallParentFunction) ; This node is disabled and will not be called.\nDrag off pins to build functionality.
)

(event EventOnGameStateReplicated
  (bind _frontlinehudwidget (Variables|Default|GetFrontlineHUDWidget))
  (bind _pushhudwidget (Variables|Default|GetPushHUDWidget))
  (|CallParentFunction)
  (Utilities|IsValid _pushhudwidget
    (:Is%20Valid
      (Widget|RemovefromParent _pushhudwidget))
    (:Is%20Not%20Valid
      _))
  (Utilities|IsValid _frontlinehudwidget
    (:Is%20Valid
      (Widget|RemovefromParent _frontlinehudwidget))
    (:Is%20Not%20Valid
      _))
  (bind _returnvalue (UserInterface|CreateWidget "/Game/Mordhau/Maps/Chasm/Chasm_sharedassets/CTF/CTFWidget.CTFWidget_C" (Game|GetPlayerController 0)))
  (bind _output_get (Variables|Default|SetWidgetCTF _returnvalue))
  (UserInterface|Viewport|AddtoViewport _output_get -4)
  (if (Variables|Default|GetIsHUDMinimal)
    (Widget|SetVisibility _output_get "Hidden")))

(event EventHideMainMenu
  (bind _widgetctf (Variables|Default|GetWidgetCTF))
  (|CallParentFunction)
  (Utilities|IsValid _widgetctf
    (:Is%20Valid
      (Widget|SetVisibility _widgetctf "Visible"))))

(event EventShowMainMenu
  (params (ArmoryState :type E_ArmoryStates%20Enum :default "NewEnumerator0"))
  (bind _widgetctf (Variables|Default|GetWidgetCTF))
  (|CallParentFunction ArmoryState)
  (Utilities|IsValid _widgetctf
    (:Is%20Valid
      (Widget|SetVisibility _widgetctf "Hidden"))))

(event EventUseMinimalHUD
  (bind _widgetctf (Variables|Default|GetWidgetCTF))
  (|CallParentFunction)
  (Utilities|IsValid _widgetctf
    (:Is%20Valid
      (Widget|SetVisibility _widgetctf "Hidden"))))

(event EventUseFullHUD
  (bind _widgetctf (Variables|Default|GetWidgetCTF))
  (|CallParentFunction)
  (Utilities|IsValid _widgetctf
    (:Is%20Valid
      (Widget|SetVisibility _widgetctf "Visible"))))

(fn ConstructionScript
  (|CallParentFunction))